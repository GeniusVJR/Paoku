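; Player character for a three-lane parkour runner that moves forward automatically, jumps, and switches lanes with A/D.
; Key presses fill a two-slot buffer that Tick consumes, starting a lane change when the target lane is valid.
; A timeline lerps Y with a swept move and reverses if blocked, committing the lane only on forward completion.
; Falling too low restarts the level immediately; HitToDeath ragdolls the mesh, then restarts after a delay.
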(event `self.ReceiveTick`
  (params (DeltaSeconds :type "Float (single-precision)"))
  ;[1 1 1] Tick
  (if (not (`self.IsDead`))
    (`self.CheckFailToDeath`)
    (`self.HandleChangeLane`)
    (`self.AddMovementInput` (`KismetMathLibrary.GetForwardVector` (`self.GetControlRotation`)))))

(event `Key|A`
  (params (Key :type "Key Structure" :default "AnyKey"))
  ;[1 1 1] 按键缓冲处理
  (:`Pressed`
    (set `self.NewKey` -1)
    (if (< (`KismetArrayLibrary.Array_Length` (`self.KeyBuffer`)) 2) :!label _label
      (`KismetArrayLibrary.Array_Add` (`self.KeyBuffer`) (`self.NewKey`)))))

(event `Key|D`
  (params (Key :type "Key Structure" :default "AnyKey"))
  ;[1 1 1] 按键缓冲处理
  (:`Pressed`
    (set `self.NewKey` 1)
    (goto _label)))

(event `CheckFailToDeath`
  (bind (_returnvalue_x _returnvalue_y _returnvalue_z) (`KismetMathLibrary.BreakVector` (`self.K2_GetActorLocation`)))
  ;[1 1 1] 检测摔死
  (if (`NavMovementComponent.IsFalling` (`self.CharacterMovement`))
    (if (< _returnvalue_z -300.0)
      (`KismetSystemLibrary.ExecuteConsoleCommand` "RestartLevel"))))

(event `HandleChangeLane`
  (bind _newlane (`self.NewLane`))
  ;[1 1 1] 计算目标跑道
  (if (`self.IsChangeLane`)
    _
    (elif (> (`KismetArrayLibrary.Array_Length` (`self.KeyBuffer`)) 0)
      (set `self.NewLane` (+ (`self.CurrentLane`) (`KismetArrayLibrary.Array_Get` (`self.KeyBuffer`))))
      (`KismetArrayLibrary.Array_Remove` (`self.KeyBuffer`))
      (bind _output_get (set `self.IsChangeLane` (and (<= _newlane 2) (>= _newlane 0))))
      (if _output_get
        (`self.StartChangeLane`)))))

(event `InputAction|Jump`
  (params (Key :type "Key Structure" :default "AnyKey"))
  ;[1 1 1] 跳跃
  (:`Pressed`
    (if (not (`self.IsDead`))
      (`self.Jump`))))

(event `StartChangeLane`
  (bind (_returnvalue_x _returnvalue_y _returnvalue_z) (`KismetMathLibrary.BreakVector` (`self.K2_GetActorLocation`)))
  (bind _lanes (`self.Lanes`))
  ;[1 1 1] 变道
  (bind (_direction _alpha) (`Timeline|ChangeLaneTimeLane` :!via `PlayFromStart` :!label _label_2)
    (:`Update`
      (bind (_sweephitresult _returnvalue) (`self.K2_SetActorLocation` (`KismetMathLibrary.MakeVector` _returnvalue_x (`KismetMathLibrary.Lerp` (`KismetArrayLibrary.Array_Get` _lanes (`self.CurrentLane`)) (`KismetArrayLibrary.Array_Get` _lanes (`self.NewLane`)) _alpha) _returnvalue_z) true))
      (if (not _returnvalue)
        (goto _label_2 :!via `Reverse`)))
    (:`Finished`
      (set `self.IsChangeLane` false)
      (switch `ETimelineDirection` _direction
        (:`Forward`
          (set `self.CurrentLane` (`self.NewLane`)))))))

(event `HitToDeath`
  (bind _mesh (`self.Mesh`))
  ;[1 1 1] 撞死
  (set `self.IsDead` true)
  (`PrimitiveComponent.SetSimulatePhysics` _mesh true)
  (`PrimitiveComponent.SetCollisionEnabled` _mesh "QueryAndPhysics")
  (`ActorComponent.SetActive` (`self.CharacterMovement`) false false)
  (`KismetSystemLibrary.Delay` 2.0)
  (`KismetSystemLibrary.ExecuteConsoleCommand` "RestartLevel"))

(fn `UserConstructionScript`)