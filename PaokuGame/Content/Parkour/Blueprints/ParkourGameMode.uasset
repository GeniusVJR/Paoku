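; Game mode for a lane-based parkour runner that builds the track and keeps the coin count.
; On BeginPlay it spawns a short run of flat tiles followed by a long run of random tiles, chaining each through the previous tile's next-floor transform.
; It then copies lane data from the first tile found to the first character found.
; IncrementCoin adds to the total and prints it.
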(event `self.ReceiveBeginPlay`
  (`|ExecutionSequence`
    (:`then_0`
      (for _ (range 7)
        (`self.AddTile` "/Game/Parkour/Blueprints/BP_Tile_Child_Flat.BP_Tile_Child_Flat_C")))
    (:`then_1`
      (for _ (range 7 101)
        (`self.AddTile` "/Game/Parkour/Blueprints/BP_Tile_Child_Random.BP_Tile_Child_Random_C")))
    (:`then_2`
      (bind _outactors (`GameplayStatics.GetAllActorsOfClass` "/Game/Parkour/Blueprints/BP_Tile.BP_Tile_C"))
      (bind _retval (`/Game/Parkour/Blueprints/BP_Tile.GetLanes` (`KismetArrayLibrary.Array_Get` _outactors)))
      (bind _outactors_2 (`GameplayStatics.GetAllActorsOfClass` "/Game/Parkour/Blueprints/BP_Character.BP_Character_C"))
      (set `/Game/Parkour/Blueprints/BP_Character.Lanes` _retval (`KismetArrayLibrary.Array_Get` _outactors_2)))))

(event `IncrementCoin`
  (params (NewParam :type Integer))
  ;[1 1 1] 加金币
  (bind _output_get (set `self.CoinNum` (+ NewParam (`self.CoinNum`))))
  (`KismetSystemLibrary.PrintString` (`KismetStringLibrary.Conv_IntToString` _output_get)))

(event `AddTile`
  (params (NewParam :type "/Game/Parkour/Blueprints/BP_Tile Class Reference"))
  ;[1 1 1] 生成地板
  (bind _returnvalue (`|SpawnActorFromClass` NewParam (`self.NextFloorTransform`) "Undefined" "OverrideRootScale"))
  (bind _newparam (`/Game/Parkour/Blueprints/BP_Tile.GetNextFloorTransform` _returnvalue))
  (set `self.NextFloorTransform` _newparam))

(event `AddTileWithRandom`
  ;[1 1 1] 随机生成地板
  (`self.AddTile` null))

(fn `NewFunction_0`)

(fn `NewFunction_1`)

(fn `UserConstructionScript`)