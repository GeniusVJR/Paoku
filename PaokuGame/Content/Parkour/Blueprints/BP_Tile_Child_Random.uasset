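; Parkour tile child Blueprint that randomizes the layout of its three component slots and its coin placement in the construction script.
; A weighted roll usually yields all floor or one obstacle, and rarely two obstacles with a single floor slot.
; A helper picks each obstacle as an empty class, blocker or wall.
; After spawning the components, it flags one random slot for coins and calls PlaceAllCoins.
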(fn `RandomTileComponentClassWithoutFloor`
  (returns (TileComponentClass :type "/Game/Parkour/Blueprints/BP_Tile_Component Class Reference"))
  (locals (NewLocalVar_0 :type "/Game/Parkour/Blueprints/BP_Tile_Component Class Reference"))
  (switch `int` (`KismetMathLibrary.RandomInteger` 3)
    (:`0`
      (set `local.NewLocalVar_0` null))
    (:`1`
      (set `local.NewLocalVar_0` "/Game/Parkour/Blueprints/BP_Tile_Component_Child_Blocker.BP_Tile_Component_Child_Blocker_C"))
    (:`2`
      (set `local.NewLocalVar_0` "/Game/Parkour/Blueprints/BP_Tile_Component_Child_Wall.BP_Tile_Component_Child_Wall_C")))
  (return (`local.NewLocalVar_0`)))

(fn `UserConstructionScript`
  (locals (NewLocalVar_1 :type Integer :default 0) (BlockerIndex :type Integer :default 0) (NewLocalVar_2 :type Integer :default 0))
  (`parent.UserConstructionScript`)
  (`|ExecutionSequence`
    (:`then_0`
      (bind _output_get (set `local.NewLocalVar_1` (`KismetMathLibrary.RandomInteger` 10)))
      ;[1 1 1] 50%的概率无障碍物
      (if (<= _output_get 4)
        (for _index (range 3)
          (`KismetArrayLibrary.Array_Set` (`self.TileComponentClasses`) _index "/Game/Parkour/Blueprints/CP_Tile_Component_Child_Floor.CP_Tile_Component_Child_Floor_C"))
        (else
          ;[1 1 1] 40%的概率一个障碍物
          (if (<= _output_get 8)
            (bind _output_get_2 (set `local.BlockerIndex` (`KismetMathLibrary.RandomInteger` 3)))
            (for _index_2 (range 3)
              (if (== _index_2 _output_get_2)
                (bind _tilecomponentclass (`self.RandomTileComponentClassWithoutFloor`))
                (`KismetArrayLibrary.Array_Set` (`self.TileComponentClasses`) _index_2 _tilecomponentclass)
                (else
                  (`KismetArrayLibrary.Array_Set` (`self.TileComponentClasses`) _index_2 "/Game/Parkour/Blueprints/CP_Tile_Component_Child_Floor.CP_Tile_Component_Child_Floor_C"))))
            (else
              (bind _output_get_3 (set `local.BlockerIndex` (`KismetMathLibrary.RandomInteger` 3)))
              (for _index_3 (range 3)
                (if (== _index_3 _output_get_3)
                  (`KismetArrayLibrary.Array_Set` (`self.TileComponentClasses`) _index_3 "/Game/Parkour/Blueprints/CP_Tile_Component_Child_Floor.CP_Tile_Component_Child_Floor_C")
                  (else
                    (bind _tilecomponentclass_2 (`self.RandomTileComponentClassWithoutFloor`))
                    (`KismetArrayLibrary.Array_Set` (`self.TileComponentClasses`) _index_3 _tilecomponentclass_2)))))))))
    (:`then_1`
      (`self.SpawnAllTileComponents`))
    (:`then_2`
      (bind _output_get_4 (set `local.NewLocalVar_2` (`KismetMathLibrary.RandomInteger` 3)))
      (for _index_4 (range 3)
        (`KismetArrayLibrary.Array_Set` (`self.IsHadPlacedCoins`) _index_4 (== _index_4 _output_get_4)))
      (`self.PlaceAllCoins`))))