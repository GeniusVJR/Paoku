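; BP_Tile is a three-lane floor segment for an endless parkour runner that exposes its lane Y positions and the attach transform for the next tile.
; Left, center and right Child Actor components are gathered into an array, given per-lane classes, and told to place coins on flagged lanes.
; When BP_Character overlaps its box, it asks ParkourGameMode to add a random tile, then destroys itself two seconds later unless the character is dead.
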(event `self.Box.OnComponentBeginOverlap`
  (params (OverlappedComponent :type "PrimitiveComponent Object Reference") (OtherActor :type "Actor Object Reference") (OtherComp :type "PrimitiveComponent Object Reference") (OtherBodyIndex :type Integer) (bFromSweep :type Boolean) (SweepResult :type "HitResult Structure (by ref)"))
  (bind _asbp_character (cast `/Game/Parkour/Blueprints/BP_Character` OtherActor))
  (bind _asparkour_game_mode (cast `/Game/Parkour/Blueprints/ParkourGameMode` (`GameplayStatics.GetGameMode`)))
  (`/Game/Parkour/Blueprints/ParkourGameMode.AddTileWithRandom` _asparkour_game_mode)
  (`KismetSystemLibrary.Delay` 2.0)
  (if (not (`/Game/Parkour/Blueprints/BP_Character.IsDead` _asbp_character))
    (`self.K2_DestroyActor`)))

(fn `CreateTileComponentArray`
  (set `self.TileComponents` (`|MakeArray` (`self.LeftTileComponent`) (`self.CenterTileComponent`) (`self.RightTileComponent`))))

(fn `GetLanes`
  (returns (RetVal :type "Array of Float (double-precision)"))
  (bind (_returnvalue_x _returnvalue_y) (`KismetMathLibrary.BreakVector` (`SceneComponent.K2_GetComponentLocation` (`self.RightTileComponent`))))
  (bind (_returnvalue_x_2 _returnvalue_y_2) (`KismetMathLibrary.BreakVector` (`SceneComponent.K2_GetComponentLocation` (`self.LeftTileComponent`))))
  (bind (_returnvalue_x_3 _returnvalue_y_3) (`KismetMathLibrary.BreakVector` (`SceneComponent.K2_GetComponentLocation` (`self.CenterTileComponent`))))
  (return (`|MakeArray` _returnvalue_y_2 _returnvalue_y_3 _returnvalue_y)))

(fn `GetNextFloorTransform`
  (returns (NewParam :type "Transform Structure"))
  (return (`SceneComponent.K2_GetComponentToWorld` (`self.NextFloorTileArrow`))))

(fn `PlaceAllCoins`
  (for _index (range 3)
    (if (`KismetArrayLibrary.Array_Get` (`self.IsHadPlacedCoins`) _index)
      (bind _asbp_tile_component (cast `/Game/Parkour/Blueprints/BP_Tile_Component` (`ChildActorComponent.ChildActor` (`KismetArrayLibrary.Array_Get` (`self.TileComponents`) _index))))
      (`/Game/Parkour/Blueprints/BP_Tile_Component.PlaceCoin` _asbp_tile_component))))

(fn `SpawnAllTileComponents`
  (for _index (range 3)
    (`ChildActorComponent.SetChildActorClass` (`KismetArrayLibrary.Array_Get` (`self.TileComponents`) _index) (`KismetArrayLibrary.Array_Get` (`self.TileComponentClasses`) _index))))

(fn `UserConstructionScript`
  (`self.CreateTileComponentArray`))